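; A replicated item actor that flies by projectile movement and notifies the AI controller of any overlapping actor so it can be picked up.
; Its mesh comes from a data asset, applied on the server at construction and on clients through RepNotify.
; It precomputes a landing location, runs a looping timer until landing, and has a downward trace to position a box at ground level.
; On landing, the server notifies the GameState and starts a despawn lifespan.
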(event `self.ReceiveBeginPlay`
  (bind _returnvalue (`KismetSystemLibrary.K2_SetTimerDelegate` (`|CreateDelegate` :!event `TraceOnLand`) 0.03 true))
  (set `self.TraceOnLandHandle` _returnvalue)
  (add `self.OnDestroyed` (`|CreateDelegate` :!event `ResetOnGameState`))
  (bind _returnvalue_2 (`SimpleFunctionLibrary.CalculateItemLandingLocation` self))
  (set `self.EstimatedLandingLocation` _returnvalue_2))

(event `self.Item.OnComponentBeginOverlap`
  (params (OverlappedComponent :type "PrimitiveComponent Object Reference") (OtherActor :type "Actor Object Reference") (OtherComp :type "PrimitiveComponent Object Reference") (OtherBodyIndex :type Integer) (bFromSweep :type Boolean) (SweepResult :type "HitResult Structure (by ref)"))
  (message `/Game/Blueprints/Interfaces/BPI_Interact.PickUp` (`AIBlueprintHelperLibrary.GetAIController` OtherActor) self))

(event `self.ProjectileMovement.OnProjectileStop`
  (params (ImpactResult :type "HitResult Structure (by ref)"))
  (`KismetSystemLibrary.K2_ClearAndInvalidateTimerHandle` (`self.TraceOnLandHandle`))
  (set `self.EstimatedLandingLocation` (`self.K2_GetActorLocation`))
  (`/Engine/EditorBlueprintResources/ActorMacros.Switch Has Authority`
    (:`Authority`
      (message `/Game/Blueprints/Interfaces/BPI_GameState.ItemLocationChanged` (`GameplayStatics.GetGameState`))
      (`self.SetLifeSpan` 6.0))))

(event `ResetOnGameState` :!signature `self.OnDestroyed`
  (params (Actor :type "Actor Object Reference"))
  (message `/Game/Blueprints/Interfaces/BPI_GameState.SetItemInGame` (`GameplayStatics.GetGameState`) null))

(fn `GetDataAsset`
  (returns (DataAsset :type "ItemDA Object Reference"))
  (return (`self.ItemDA`)))

(fn `GetEstimatedLandingLocation`
  (returns (ReturnValue :type "Vector Structure"))
  (return (`self.EstimatedLandingLocation`)))

(fn `GetItemGravity`
  (returns (ReturnValue :type "Float (single-precision)"))
  (return (`MovementComponent.GetGravityZ` (`self.ProjectileMovement`))))

(fn `GetLandTraceLocation`
  (returns (LocationOnLand :type "Vector Structure"))
  (return (`SceneComponent.K2_GetComponentLocation` (`self.Box`))))

(fn `OnRep_ItemDA`
  (`/Engine/EditorBlueprintResources/ActorMacros.Switch Has Authority`
    (:`Remote`
      (`StaticMeshComponent.SetStaticMesh` (`self.Item`) (`|ConvertAsset` (`ItemDA.ItemMesh` (`self.ItemDA`)))))))

(fn `TraceOnLand`
  (bind _returnvalue (`self.K2_GetActorLocation`))
  (bind _outhit (`KismetSystemLibrary.LineTraceSingle` _returnvalue (+ _returnvalue (0.0 0.0 -5000.0)) "TraceTypeQuery1"))
  (`SceneComponent.K2_SetWorldTransform` (`self.Box`) (`KismetMathLibrary.MakeTransform` (+ (`.Location` (`GameplayStatics.BreakHitResult` _outhit)) (0.0 0.0 32.0))) false true))

(fn `UserConstructionScript`
  (`/Engine/EditorBlueprintResources/ActorMacros.Switch Has Authority`
    (:`Authority`
      (`StaticMeshComponent.SetStaticMesh` (`self.Item`) (`|ConvertAsset` (`ItemDA.ItemMesh` (`self.ItemDA`))))
      (`MovementComponent.SetUpdatedComponent` (`self.ProjectileMovement`) (`self.Item`)))))