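; Base game state that holds shared match data: the play item, registered NPCs, remaining time, finish flag and winner.
; Setting the item triggers recalculation of AI path costs and their maximum, then announces it; item moves broadcast a raised location.
; AI names and genders are drawn randomly without repeats from a resettable pool, and getters expose NPC names and scores.
; It can also have every player controller destroy its client session.
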(event `/Game/Blueprints/Interfaces/BPI_GameState.SetItemInGame`
  (params (Item :type "Actor Object Reference"))
  (bind _output_get (set `self.PlayItem` Item))
  (`self.CalculateAI_CurrentPathCosts`)
  (`self.FindCurrentMaxPathCost`)
  (`self.OnItemInGame` _output_get))

(event `/Game/Blueprints/Interfaces/BPI_GameState.UpdateRemainingTime`
  (params (Time :type "Float (double-precision)"))
  (set `self.RemainingTime` Time))

(event `/Game/Blueprints/Interfaces/BPI_GameState.AddAIController`
  (params (Controller :type "/Game/Blueprints/Controllers/BP_AIController Object Reference"))
  (bind _asbase_aicharacter (cast `BaseAICharacter` (`Controller.K2_GetPawn` Controller)))
  (`KismetArrayLibrary.Array_AddUnique` (`self.NPCs`) _asbase_aicharacter))

(event `/Game/Blueprints/Interfaces/BPI_GameState.ResetAINamePool`
  (params (NamePool :type "Map of Name to EGender Enum"))
  (set `self.CurrentNamePool` NamePool))

(event `/Game/Blueprints/Interfaces/BPI_GameState.SetGameFinished`
  (params (Finished :type Boolean))
  (set `self.bGameFinshed` Finished)
  (`self.OnRep_GameFinished`))

(event `self.DestroyAllSessions`
  (for _array_element (`self.PlayerArray`)
    (bind _asbp_player_controller (cast `/Game/Blueprints/Controllers/BP_PlayerController` (`PlayerState.GetPlayerController` _array_element)))
    (`/Game/Blueprints/Controllers/BP_PlayerController.DestroySessionClient` _asbp_player_controller)))

(event `/Game/Blueprints/Interfaces/BPI_GameState.ItemLocationChanged`
  (`self.OnItemLocationChanged` (+ (`self.K2_GetActorLocation` (`self.PlayItem`)) (0.0 0.0 32.0))))

(fn `GetAI_Info`
  (returns (Names :type "Array of Name") (Scores :type "Array of Integer"))
  (locals (LocalNames :type "Array of Name") (LocalScores :type "Array of Integer"))
  (for _array_element (`self.NPCs`)
    (bind _returnvalue (message `AI_Interface.GetAI_Name` _array_element))
    (`KismetArrayLibrary.Array_Add` (`local.LocalNames`) _returnvalue)
    (bind _returnvalue_2 (message `AI_Interface.GetAI_Score` _array_element))
    (`KismetArrayLibrary.Array_Add` (`local.LocalScores`) _returnvalue_2))
  (return (`local.LocalNames`) (`local.LocalScores`)))

(fn `GetAICharacters`
  (returns (AICharacters :type "Array of BaseAICharacter Object Reference"))
  (return (`self.NPCs`)))

(fn `GetAIInfo2`
  (returns (Names :type "Array of Name") (Scores :type "Array of Integer"))
  (locals (LocalNames :type "Array of Name") (LocalScores :type "Array of Integer")))

(fn `GetAIInitProps`
  (returns (Name :type Name) (Gender :type "EGender Enum"))
  (locals (CurrentName :type Name) (Index :type Integer) (LocalGender :type "EGender Enum"))
  (bind _currentnamepool (`self.CurrentNamePool`))
  (bind _keys (`BlueprintMapLibrary.Map_Keys` _currentnamepool))
  (set `local.Index` (`.OutIndex` (`KismetArrayLibrary.Array_Random` _keys)))
  (bind _keys_2 (`BlueprintMapLibrary.Map_Keys` _currentnamepool))
  (bind _output_get (set `local.CurrentName` (`|GetArrayItem` _keys_2 (`local.Index`))))
  (set `local.LocalGender` (`BlueprintMapLibrary.Map_Find` (`self.CurrentNamePool`) _output_get))
  (`BlueprintMapLibrary.Map_Remove` (`self.CurrentNamePool`) _output_get)
  (return (`local.CurrentName`) (`local.LocalGender`)))

(fn `GetCurrentPathMaxCost`
  (returns (AICharacterToCost :type "Map of Pawn Object Reference to Float (double-precision)") (Cost :type "Float (double-precision)"))
  (return (`self.NPC_ToPathCost`) (`self.MaxPathCost`)))

(fn `GetRemainingTime`
  (returns (Time :type "Float (double-precision)"))
  (return (`self.RemainingTime`)))

(fn `GetWinner`
  (returns (Name :type Name) (Score :type Integer))
  (return (`self.WinnerName`) (`self.WinnerScore`)))

(fn `IsItemInGame`
  (returns (InGame :type Boolean))
  (return (`KismetSystemLibrary.IsValid` (`self.PlayItem`))))

(fn `UserConstructionScript`)