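; BP_AICharacter is an AI character with a replicated name, gender and walk speed setup.
; On BeginPlay the server pulls name and gender from TestGameStateBase and applies MoveSpeed, randomized within min/max when left at zero.
; RepNotifies push the name to the nameplate widget and swap Manny or Quinn mesh and AnimBP by gender.
; The construction script runs the same mesh correction.
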(event `self.ReceiveBeginPlay`
  (bind _movespeed (`self.MoveSpeed`))
  (`/Engine/EditorBlueprintResources/ActorMacros.Switch Has Authority`
    (:`Authority`
      (bind _astest_game_state_base (cast `TestGameStateBase` (`GameplayStatics.GetGameState`)))
      (bind (_name _gender) (`TestGameStateBase.GetAI_InitInfo` _astest_game_state_base))
      (set `self.Name` _name)
      (set `self.Gender` _gender)
      (bind _output_get (set `self.MoveSpeed` (`KismetMathLibrary.SelectFloat` (`KismetMathLibrary.RandomFloatInRange` (`self.MinMoveSpeed`) (`self.MaxMoveSpeed`)) _movespeed (== _movespeed 0.0))))
      (set `CharacterMovementComponent.MaxWalkSpeed` _output_get (`self.CharacterMovement`))
      (`self.OnRep_Name`))))

(fn `CorrectSkeletalMesh`
  (bind _gender (`self.Gender`))
  (`SkeletalMeshComponent.SetSkeletalMeshAsset` (`self.Mesh`) (select `EGender` _gender :`Male` "/Game/Characters/AICharacters/Meshes/SKM_Manny_Simple.SKM_Manny_Simple" :`Female` "/Game/Characters/AICharacters/Meshes/SKM_Quinn_Simple.SKM_Quinn_Simple" :!type "SkeletalMesh Object Reference"))
  (`SkeletalMeshComponent.SetAnimInstanceClass` (`self.Mesh`) (select `EGender` _gender :`Male` "/Game/Characters/AICharacters/Animations/ABP_Manny.ABP_Manny_C" :`Female` "/Game/Characters/AICharacters/Animations/ABP_Quinn.ABP_Quinn_C" :!type "Object Class Reference")))

(fn `OnRep_Gender`
  (`self.CorrectSkeletalMesh`))

(fn `OnRep_Name`
  (bind _aswb_ainame_plate (cast `/Game/Blueprints/Widgets/WB_AINamePlate` (`WidgetComponent.GetWidget` (`self.NamePlateC`))))
  (`/Game/Blueprints/Widgets/WB_AINamePlate.SetName` _aswb_ainame_plate (`KismetTextLibrary.Conv_NameToText` (`self.Name`))))

(fn `UserConstructionScript`
  (`self.CorrectSkeletalMesh`))