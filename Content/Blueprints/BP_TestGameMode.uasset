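; Game mode Blueprint that runs a timed match and drives its TestGameStateBase.
; On BeginPlay it starts a one-shot timer of GameTime length and a fast looping timer, then resets the game state's AI name pool from CurrentNamePool.
; UpdateRemainingTime pushes the match timer's remaining time to the game state, while GameEnded clears the looping timer and flags the game as finished.
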(event `self.ReceiveBeginPlay`
  (bind _returnvalue (`KismetSystemLibrary.K2_SetTimerDelegate` (`|CreateDelegate` :!event `GameEnded`) (`self.GameTime`)))
  (set `self.GameTimeHandle` _returnvalue)
  (bind _returnvalue_2 (`KismetSystemLibrary.K2_SetTimerDelegate` (`|CreateDelegate` :!event `UpdateRemainingTime`) 0.03 true))
  (set `self.RemainingTimeHandle` _returnvalue_2)
  (bind _astest_game_state_base (cast `TestGameStateBase` (`GameplayStatics.GetGameState`)))
  (bind _output_get (set `self.CurrentGameState` _astest_game_state_base))
  (`TestGameStateBase.ResetAI_NamePool` _output_get (`self.CurrentNamePool`)))

(event `UpdateRemainingTime`
  (`TestGameStateBase.UpdateRemainingTime` (`self.CurrentGameState`) (`KismetSystemLibrary.K2_GetTimerRemainingTimeHandle` (`self.GameTimeHandle`))))

(event `GameEnded`
  (`KismetSystemLibrary.K2_ClearAndInvalidateTimerHandle` (`self.RemainingTimeHandle`))
  (`TestGameStateBase.SetGameFinished` (`self.CurrentGameState`) true))

(fn `UserConstructionScript`)